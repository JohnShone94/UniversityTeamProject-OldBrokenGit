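; HealthPad is a pad that acts on the player character's health while the character stands on it.
; Capsule begin and end overlaps with TheMainGameCharacter set an Overlapped flag and toggle the health particles, which start inactive.
; While flagged, Tick runs through a one-second Delay, passes a random small integer to SetCurrentHealth on player 0, then caps health at maximum.
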(event `self.ReceiveBeginPlay`
  (`ActorComponent.SetActive` (`self.healthParticles`) false false))

(event `self.ReceiveTick`
  (params (DeltaSeconds :type "Float (single-precision)"))
  (if (`self.overlapped`)
    (`KismetSystemLibrary.Delay` 1.0)
    (bind _asthe_main_game_character (cast `TheMainGameCharacter` (`GameplayStatics.GetPlayerCharacter` 0)))
    (`TheMainGameCharacter.SetCurrentHealth` _asthe_main_game_character (`KismetMathLibrary.RandomIntegerInRange` 5 10))
    (if (>= (`TheMainGameCharacter.GetCurrentHealth` _asthe_main_game_character) (`TheMainGameCharacter.GetMaxHealth` _asthe_main_game_character))
      (`TheMainGameCharacter.SetCurrentHealth` _asthe_main_game_character (`TheMainGameCharacter.GetMaxHealth` _asthe_main_game_character)))))

(event `self.Capsule.OnComponentBeginOverlap`
  (params (OverlappedComponent :type "PrimitiveComponent Object Reference") (OtherActor :type "Actor Object Reference") (OtherComp :type "PrimitiveComponent Object Reference") (OtherBodyIndex :type Integer) (bFromSweep :type Boolean) (SweepResult :type "HitResult Structure (by ref)"))
  (cast `TheMainGameCharacter` OtherActor)
  (set `self.overlapped` true)
  (`ActorComponent.SetActive` (`self.healthParticles`) true false))

(event `self.Capsule.OnComponentEndOverlap`
  (params (OverlappedComponent :type "PrimitiveComponent Object Reference") (OtherActor :type "Actor Object Reference") (OtherComp :type "PrimitiveComponent Object Reference") (OtherBodyIndex :type Integer))
  (cast `TheMainGameCharacter` OtherActor)
  (set `self.overlapped` false)
  (`ActorComponent.SetActive` (`self.healthParticles`) false false))

(fn `UserConstructionScript`)