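; Enemy actor that turns toward and shoots the player character on sight, and is destroyed when hit by a player projectile.
; Pawn sensing triggers the rotation and a projectile spawn with a forward impulse, throttled by a boolean and delay.
; BeginPlay gathers three patrol points and picks one at random, but the timeline logic that would lerp between them never runs.
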(event `self.PawnSensing.OnSeePawn`
  (params (Pawn :type "Pawn Object Reference"))
  ;[1 1 1] Look at and shoot
  (bind _asbp_the_main_game_character (cast `/Game/Blueprints/Character/bp_TheMainGameCharacter` Pawn))
  (`|ExecutionSequence`
    (:`then_0`
      (`self.K2_SetActorRotation` (`KismetMathLibrary.FindLookAtRotation` (`self.K2_GetActorLocation`) (`self.K2_GetActorLocation` _asbp_the_main_game_character))))
    (:`then_1`
      (if (`self.SpawnProjectile`)
        (bind _returnvalue (`|SpawnActorFromClass` "/Game/Blueprints/AI/EnemyProjectile.EnemyProjectile_C" (`SceneComponent.K2_GetComponentToWorld` (`self.ProjectileSpawnLocation`)) "Undefined" "OverrideRootScale"))
        (`PrimitiveComponent.AddImpulse` (`/Game/Blueprints/AI/EnemyProjectile.Sphere` _returnvalue) (* (`SceneComponent.GetForwardVector` (`self.Cube`)) (`self.ShootAmount`)) "None" true)
        (set `self.SpawnProjectile` false)
        (`KismetSystemLibrary.Delay` 1.5)
        (set `self.SpawnProjectile` true)))))

(event `self.ReceiveBeginPlay`
  ;[1 1 1] Set Partrol Points
  (set `self.PatrolPoints` (`|MakeArray` (`SceneComponent.K2_GetComponentLocation` (`self.MovePosition1`)) (`SceneComponent.K2_GetComponentLocation` (`self.MovePosition2`)) (`SceneComponent.K2_GetComponentLocation` (`self.MovePosition3`))))
  (`self.GetRandomLocation`))

(event `self.ReceiveHit`
  (params (MyComp :type "PrimitiveComponent Object Reference") (Other :type "Actor Object Reference") (OtherComp :type "PrimitiveComponent Object Reference") (bSelfMoved :type Boolean) (HitLocation :type "Vector Structure") (HitNormal :type "Vector Structure") (NormalImpulse :type "Vector Structure") (Hit :type "HitResult Structure (by ref)"))
  ;[1 1 1] removes health if a bullet makes contact with the player.
  (cast `TheMainGameProjectile` Other)
  (`self.K2_DestroyActor`))

(fn `GetRandomLocation`
  (set `self.CurrentPatrolPoints` (`KismetMathLibrary.RandomInteger` (`KismetArrayLibrary.Array_Length` (`self.PatrolPoints`)))))

(fn `UserConstructionScript`)