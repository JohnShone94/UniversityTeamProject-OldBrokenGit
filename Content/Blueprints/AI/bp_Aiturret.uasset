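; AI turret enemy that turns toward the main character when pawn sensing sees it and fires impulse-driven projectiles on a 1.5-second cooldown.
; When its Active flag is set, a delayed Tick check plays a timeline that lerps the cube to its Mid transform, then enables sensing.
; It starts with a small random health, loses one per player projectile hit, and is destroyed when Tick finds health depleted.
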(event `self.PawnSensing.OnSeePawn`
  (params (Pawn :type "Pawn Object Reference"))
  (bind _asthe_main_game_character (cast `TheMainGameCharacter` Pawn))
  (`|ExecutionSequence`
    (:`then_0`
      (`self.K2_SetActorRotation` (`KismetMathLibrary.FindLookAtRotation` (`self.K2_GetActorLocation`) (`self.K2_GetActorLocation` _asthe_main_game_character))))
    (:`then_1`
      (if (`self.SpawnProjectile`)
        (bind _returnvalue (`|SpawnActorFromClass` "/Game/Blueprints/AI/EnemyProjectile.EnemyProjectile_C" (`SceneComponent.K2_GetComponentToWorld` (`self.ProjectileSpawnLocation`)) "Undefined" "OverrideRootScale"))
        (`PrimitiveComponent.AddImpulse` (`/Game/Blueprints/AI/EnemyProjectile.Sphere` _returnvalue) (* (`SceneComponent.GetForwardVector` (`self.Cube`)) (`self.ShootAmount`)) "None" true)
        (set `self.SpawnProjectile` false)
        (`KismetSystemLibrary.Delay` 1.5)
        (set `self.SpawnProjectile` true)))))

(event `Activate`
  ;[1 1 1] Activates a timeline to transform the AI into its starting position
  (bind (_direction _newtrack_0) (`Timeline|Timeline_0` :!via `PlayFromStart`)
    (:`Update`
      (`SceneComponent.K2_SetRelativeTransform` (`self.Cube`) (`KismetMathLibrary.TLerp` (`SceneComponent.GetRelativeTransform` (`self.Cube`)) (`self.Mid`) _newtrack_0) true false)
      (`KismetSystemLibrary.Delay` 0.75)
      (`PawnSensingComponent.SetSensingUpdatesEnabled` (`self.PawnSensing`) true))))

(event `self.ReceiveBeginPlay`
  ;[1 1 1] Health System
  (set `self.Health` (`KismetMathLibrary.RandomIntegerInRange` 3 6)))

(event `self.ReceiveHit`
  (params (MyComp :type "PrimitiveComponent Object Reference") (Other :type "Actor Object Reference") (OtherComp :type "PrimitiveComponent Object Reference") (bSelfMoved :type Boolean) (HitLocation :type "Vector Structure") (HitNormal :type "Vector Structure") (NormalImpulse :type "Vector Structure") (Hit :type "HitResult Structure (by ref)"))
  ;[1 1 1] removes health if a bullet makes contact with the player.
  (cast `TheMainGameProjectile` Other)
  (set `self.Health` (+ (`self.Health`) -1)))

(event `self.ReceiveTick`
  (params (DeltaSeconds :type "Float (single-precision)"))
  (`|ExecutionSequence`
    (:`then_0`
      ;[1 1 1] Activates the AI
      (`KismetSystemLibrary.Delay` 3.0)
      (if (`self.Active`)
        (`self.Activate`)))
    (:`then_1`
      ;[1 1 1] Runs the check health function
      (`self.CheckHealth`))))

(event `CheckHealth`
  ;[1 1 1] removes health if a bullet makes contact with the player.
  (if (<= (`self.Health`) 0)
    (`self.K2_DestroyActor`)))

(fn `UserConstructionScript`)