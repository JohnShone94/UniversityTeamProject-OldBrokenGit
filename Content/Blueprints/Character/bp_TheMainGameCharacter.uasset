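; Main player character Blueprint that creates the HUD and handles interaction, pause, flashlight and projectile damage.
; Interact opens a paused world-selector UI at the portal dial-up or collects overlapping power capsules, gated by overlap flags.
; Pause swaps widgets and switches to UI-only input, while enemy projectile hits pass a random negative amount to SetCurrentHealth.
; Hard-coded keys toggle the spotlight, load the save and open the example map.
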(event `Key|L`
  (params (Key :type "Key Structure" :default "AnyKey"))
  (:`Pressed`
    (`GameplayStatics.OpenLevel` "FirstPersonExampleMap")))

(event `self.ReceiveBeginPlay`
  (bind _returnvalue (`|CreateWidget` "/Game/Blueprints/HUD.HUD_C"))
  (`UserWidget.AddToViewport` _returnvalue 0))

(event `InputAction|Interact`
  (params (Key :type "Key Structure" :default "AnyKey"))
  (bind _returnvalue (`GameplayStatics.GetPlayerController` 0))
  ;[1 1 1] Allows interaction with the portal dialup
  (:`Pressed`
    (if (`self.GetIsOverlappingComp`)
      (`WidgetLayoutLibrary.RemoveAllWidgets`)
      (bind _returnvalue_2 (`|CreateWidget` "/Game/Blueprints/WorldSelector.WorldSelector_C"))
      (`UserWidget.AddToViewport` _returnvalue_2 0)
      (set `PlayerController.bShowMouseCursor` true _returnvalue)
      (`WidgetBlueprintLibrary.SetInputMode_UIOnlyEx` _returnvalue)
      (`GameplayStatics.SetGamePaused` true))))

(event `InputAction|Interact`
  (params (Key :type "Key Structure" :default "AnyKey"))
  ;[1 1 1] Allows interaction with the wall unit
  (:`Pressed`
    (if (`self.GetIsOverlappingPower`)
      (for _array_element (`PrimitiveComponent.GetOverlappingActors` (`self.CapsuleComponent`) null)
        (bind _asbp_power_capsule (cast `/Game/Blueprints/bp_PowerCapsule` _array_element))
        (`/Game/Blueprints/bp_PowerCapsule.Collect` _asbp_power_capsule)))))

(event `InputAction|LaunchPauseMenu`
  (params (Key :type "Key Structure" :default "AnyKey"))
  ;[1 1 1] Launches the pause menu
  (:`Pressed`
    (set `PlayerController.bShowMouseCursor` true (`GameplayStatics.GetPlayerController` 0))
    (`WidgetLayoutLibrary.RemoveAllWidgets`)
    (bind _returnvalue (`|CreateWidget` "/Game/Blueprints/PauseMenu.PauseMenu_C"))
    (bind _output_get (set `self.PauseMenuHUD` _returnvalue))
    (`UserWidget.AddToViewport` _output_get 0)
    (`WidgetBlueprintLibrary.SetInputMode_UIOnlyEx` (`GameplayStatics.GetPlayerController` 0) (`self.PauseMenuHUD`))
    (`GameplayStatics.SetGamePaused` true)
    (`|CreateWidget` "/Game/Blueprints/HUD.HUD_C")))

(event `Key|Z`
  (params (Key :type "Key Structure" :default "AnyKey"))
  ;[1 1 1] Loads the game
  (:`Pressed`
    (`self.RunLoadGame`)))

(event `self.ReceiveHit`
  (params (MyComp :type "PrimitiveComponent Object Reference") (Other :type "Actor Object Reference") (OtherComp :type "PrimitiveComponent Object Reference") (bSelfMoved :type Boolean) (HitLocation :type "Vector Structure") (HitNormal :type "Vector Structure") (NormalImpulse :type "Vector Structure") (Hit :type "HitResult Structure (by ref)"))
  ;[1 1 1] removes health if a bullet makes contact with the player.
  (cast `/Game/Blueprints/AI/EnemyProjectile` Other)
  (`self.SetCurrentHealth` (`KismetMathLibrary.RandomIntegerInRange` -15 -10)))

(event `Key|F`
  (params (Key :type "Key Structure" :default "AnyKey"))
  (bind _spotlight (`self.SpotLight`))
  ;[1 1 1] Interaction with the tourch
  (:`Pressed`
    (if (`self.LighOn`)
      (`LightComponent.SetIntensity` _spotlight 0.0)
      (set `self.LighOn` false)
      (else
        (`LightComponent.SetIntensity` _spotlight 100000.0)
        (set `self.LighOn` true)))))

(fn `UserConstructionScript`)