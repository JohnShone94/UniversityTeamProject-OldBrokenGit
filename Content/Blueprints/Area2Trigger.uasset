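; Trigger actor that runs a timed light flicker on bp_Light actors tagged Area2Lights when TheMainGameCharacter overlaps it.
; A Sequence starts parallel, staggered Delays over five seconds, each looping through the lights to set PointLight2.
; The lights alternate between off and bright, switching from warm to cool and back to warm, with shadow casting enabled early and disabled at the end.
; No guard prevents retriggering on later overlaps.
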(event `self.ReceiveActorBeginOverlap`
  (params (OtherActor :type "Actor Object Reference"))
  (cast `TheMainGameCharacter` OtherActor)
  (bind _outactors (`GameplayStatics.GetAllActorsWithTag` "Area2Lights"))
  (`|ExecutionSequence`
    (:`then_0`
      (for _array_element _outactors
        (bind _asbp_light (cast `/Game/Blueprints/bp_Light` _array_element))
        (`LightComponent.SetIntensity` (`/Game/Blueprints/bp_Light.PointLight2` _asbp_light) 0.0)))
    (:`then_1`
      (`KismetSystemLibrary.Delay` 1.0)
      (for _array_element_2 _outactors
        (bind _asbp_light_2 (cast `/Game/Blueprints/bp_Light` _array_element_2))
        (bind _pointlight2 (`/Game/Blueprints/bp_Light.PointLight2` _asbp_light_2))
        (`LightComponent.SetIntensity` _pointlight2 100000.0)
        (`LightComponent.SetTemperature` _pointlight2 1700.0)
        (`LightComponentBase.SetCastShadows` _pointlight2 true)))
    (:`then_2`
      (`KismetSystemLibrary.Delay` 2.0)
      (for _array_element_3 _outactors
        (bind _asbp_light_3 (cast `/Game/Blueprints/bp_Light` _array_element_3))
        (`LightComponent.SetIntensity` (`/Game/Blueprints/bp_Light.PointLight2` _asbp_light_3) 0.0)))
    (:`then_3`
      (`KismetSystemLibrary.Delay` 3.0)
      (for _array_element_4 _outactors
        (bind _asbp_light_4 (cast `/Game/Blueprints/bp_Light` _array_element_4))
        (bind _pointlight2_2 (`/Game/Blueprints/bp_Light.PointLight2` _asbp_light_4))
        (`LightComponent.SetIntensity` _pointlight2_2 100000.0)
        (`LightComponent.SetTemperature` _pointlight2_2 8000.0)))
    (:`then_4`
      (`KismetSystemLibrary.Delay` 4.0)
      (for _array_element_5 _outactors
        (bind _asbp_light_5 (cast `/Game/Blueprints/bp_Light` _array_element_5))
        (`LightComponent.SetIntensity` (`/Game/Blueprints/bp_Light.PointLight2` _asbp_light_5) 0.0)))
    (:`then_5`
      (`KismetSystemLibrary.Delay` 5.0)
      (for _array_element_6 _outactors
        (bind _asbp_light_6 (cast `/Game/Blueprints/bp_Light` _array_element_6))
        (bind _pointlight2_3 (`/Game/Blueprints/bp_Light.PointLight2` _asbp_light_6))
        (`LightComponent.SetIntensity` _pointlight2_3 100000.0)
        (`LightComponent.SetTemperature` _pointlight2_3 1700.0)
        (`LightComponentBase.SetCastShadows` _pointlight2_3 false)))))

(fn `UserConstructionScript`)