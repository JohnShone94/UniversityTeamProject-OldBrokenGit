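; Power pickup actor that activates on BeginPlay and animates a point light with a rising, sawtooth-like intensity.
; Tick raises the intensity by a fixed step each frame and resets it on exactly matching the maximum, so the ramp is frame-rate dependent.
; The reset branch passes through a Delay that does not pause later increments.
; Overlap only re-applies the current active state, with no collection logic here.
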(event `self.ReceiveBeginPlay`
  (`self.SetActive` true))

(event `self.ReceiveActorBeginOverlap`
  (params (OtherActor :type "Actor Object Reference"))
  (`self.SetActive` (`self.IsActive`)))

(event `self.ReceiveTick`
  (params (DeltaSeconds :type "Float (single-precision)"))
  (if (== (`self.intencity`) (`self.mxIntencity`))
    (set `self.intencity` 1000.0)
    (`KismetSystemLibrary.Delay` 2.0)
    (else
      (set `self.intencity` (+ (`self.intencity`) 1000.0))))
  (`LightComponent.SetIntensity` (`self.PointLight`) (`self.intencity`)))

(fn `UserConstructionScript`)