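; Power capsule pickup that gives the player power and triggers an alarm in its tagged area when collected.
; Overlap flags the character as near power and sets its PlayerArea to the capsule's AreaTag.
; Collect hides the capsule, plays sparks, sets the player's power and sets tagged doors closed, then after a delay activates tagged turrets.
; AreaLighting uses staggered Sequence delays to flash tagged lights red and white, ending on red.
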(event `self.ReceiveBeginPlay`
  ;[1 1 1] Setsup the power capsuls when the map loads
  (`ActorComponent.SetActive` (`self.PowerCapsule`) true false)
  (`ActorComponent.SetActive` (`self.sparks`) false false)
  (set `self.power` (`self.PowerAmount`)))

(event `self.ReceiveActorBeginOverlap`
  (params (OtherActor :type "Actor Object Reference"))
  ;[1 1 1] On begin overlap and on end overlap
  (bind _asthe_main_game_character (cast `TheMainGameCharacter` OtherActor))
  (`KismetSystemLibrary.PrintString` "casted")
  (`TheMainGameCharacter.SetIsOverlappingPower` _asthe_main_game_character true)
  (bind _asbp_the_main_game_character (cast `/Game/Blueprints/Character/bp_TheMainGameCharacter` (`GameplayStatics.GetPlayerCharacter` 0)))
  (set `/Game/Blueprints/Character/bp_TheMainGameCharacter.PlayerArea` (`self.Area Tag`) _asbp_the_main_game_character))

(event `self.ReceiveActorEndOverlap`
  (params (OtherActor :type "Actor Object Reference"))
  ;[1 1 1] On begin overlap and on end overlap
  (bind _asthe_main_game_character (cast `TheMainGameCharacter` OtherActor))
  (`KismetSystemLibrary.PrintString` "uncasted")
  (`TheMainGameCharacter.SetIsOverlappingPower` _asthe_main_game_character false)
  (bind _asbp_the_main_game_character (cast `/Game/Blueprints/Character/bp_TheMainGameCharacter` (`GameplayStatics.GetPlayerCharacter` 0)))
  (set `/Game/Blueprints/Character/bp_TheMainGameCharacter.PlayerArea` "None" _asbp_the_main_game_character))

(event `Collect`
  (bind _area_tag (`self.Area Tag`))
  ;[1 1 1] Collects the power
  (bind _asthe_main_game_character (cast `TheMainGameCharacter` (`GameplayStatics.GetPlayerCharacter` 0)))
  (`SceneComponent.SetVisibility` (`self.PowerCapsule`) false false)
  (`TheMainGameCharacter.SetCurrentPower` _asthe_main_game_character (`self.PowerAmount`))
  (`ActorComponent.SetActive` (`self.sparks`) true false)
  (`PrimitiveComponent.SetCollisionEnabled` (`self.Box`) "NoCollision")
  (`TheMainGameCharacter.SetIsOverlappingPower` _asthe_main_game_character false)
  (`self.ActivateDoor` _area_tag)
  (`KismetSystemLibrary.Delay` 2.0)
  (`self.AreaLighting` _area_tag)
  (`self.ActivateEnemy` _area_tag)
  (`ActorComponent.SetActive` (`self.sparks`) false false))

(event `ActivateEnemy`
  (params (`Area Tag` :type Name))
  (bind _outactors (`GameplayStatics.GetAllActorsWithTag` `Area Tag`))
  (for _array_element _outactors
    (bind _asbp_aiturret (cast `/Game/Blueprints/AI/bp_Aiturret` _array_element))
    (set `/Game/Blueprints/AI/bp_Aiturret.Active` true _asbp_aiturret)))

(event `ActivateDoor`
  (params (`Area Tag` :type Name))
  (bind _outactors (`GameplayStatics.GetAllActorsWithTag` `Area Tag`))
  (for _array_element _outactors
    (bind _asbp_door (cast `/Game/Blueprints/bp_Door` _array_element))
    (set `/Game/Blueprints/bp_Door.doorOpen` false _asbp_door)))

(event `AreaLighting`
  (params (`Area Tag` :type Name))
  (bind _outactors (`GameplayStatics.GetAllActorsWithTag` `Area Tag`))
  (`|ExecutionSequence`
    (:`then_0`
      (for _array_element _outactors
        (`|ExecutionSequence`
          (:`then_0`
            (bind _asbp_light (cast `/Game/Blueprints/bp_Light` _array_element))
            (`LightComponent.SetIntensity` (`/Game/Blueprints/bp_Light.PointLight2` _asbp_light) 0.0))
          (:`then_1`
            (bind _asbp_warning_light (cast `/Game/Blueprints/bp_WarningLight` _array_element))
            (`LightComponent.SetIntensity` (`/Game/Blueprints/bp_WarningLight.SpotLight1` _asbp_warning_light) 0.0)
            (`LightComponent.SetIntensity` (`/Game/Blueprints/bp_WarningLight.SpotLight` _asbp_warning_light) 0.0)))))
    (:`then_1`
      (`KismetSystemLibrary.Delay` 1.0)
      (for _array_element_2 _outactors
        (`|ExecutionSequence`
          (:`then_0`
            (bind _asbp_light_2 (cast `/Game/Blueprints/bp_Light` _array_element_2))
            (bind _pointlight2 (`/Game/Blueprints/bp_Light.PointLight2` _asbp_light_2))
            (`LightComponent.SetIntensity` _pointlight2 100000.0)
            (`LightComponent.SetLightColor` _pointlight2 (struct :`R` 1.0 :`A` 1.0) true)
            (`LightComponentBase.SetCastShadows` _pointlight2 true))
          (:`then_1`
            (bind _asbp_warning_light_2 (cast `/Game/Blueprints/bp_WarningLight` _array_element_2))
            (bind _spotlight (`/Game/Blueprints/bp_WarningLight.SpotLight` _asbp_warning_light_2))
            (`LightComponent.SetIntensity` _spotlight 100000.0)
            (`LightComponent.SetIntensity` (`/Game/Blueprints/bp_WarningLight.SpotLight1` _asbp_warning_light_2) 100000.0)
            (`LightComponent.SetLightColor` _spotlight (struct :`R` 1.0 :`A` 1.0) true)
            (`LightComponent.SetLightColor` (`/Game/Blueprints/bp_WarningLight.SpotLight1` _asbp_warning_light_2) (struct :`R` 1.0 :`A` 1.0) true)
            (`LightComponentBase.SetCastShadows` _spotlight true)
            (`LightComponentBase.SetCastShadows` (`/Game/Blueprints/bp_WarningLight.SpotLight1` _asbp_warning_light_2) true)))))
    (:`then_2`
      (`KismetSystemLibrary.Delay` 2.0)
      (for _array_element_3 _outactors
        (`|ExecutionSequence`
          (:`then_0`
            (bind _asbp_light_3 (cast `/Game/Blueprints/bp_Light` _array_element_3))
            (`LightComponent.SetIntensity` (`/Game/Blueprints/bp_Light.PointLight2` _asbp_light_3) 0.0))
          (:`then_1`
            (bind _asbp_warning_light_3 (cast `/Game/Blueprints/bp_WarningLight` _array_element_3))
            (`LightComponent.SetIntensity` (`/Game/Blueprints/bp_WarningLight.SpotLight1` _asbp_warning_light_3) 0.0)
            (`LightComponent.SetIntensity` (`/Game/Blueprints/bp_WarningLight.SpotLight` _asbp_warning_light_3) 0.0)))))
    (:`then_3`
      (`KismetSystemLibrary.Delay` 3.0)
      (for _array_element_4 _outactors
        (`|ExecutionSequence`
          (:`then_0`
            (bind _asbp_light_4 (cast `/Game/Blueprints/bp_Light` _array_element_4))
            (bind _pointlight2_2 (`/Game/Blueprints/bp_Light.PointLight2` _asbp_light_4))
            (`LightComponent.SetIntensity` _pointlight2_2 100000.0)
            (`LightComponent.SetLightColor` _pointlight2_2 (struct :`R` 1.0 :`G` 1.0 :`B` 1.0 :`A` 1.0) true))
          (:`then_1`
            (bind _asbp_warning_light_4 (cast `/Game/Blueprints/bp_WarningLight` _array_element_4))
            (bind _spotlight_2 (`/Game/Blueprints/bp_WarningLight.SpotLight` _asbp_warning_light_4))
            (`LightComponent.SetIntensity` _spotlight_2 100000.0)
            (`LightComponent.SetIntensity` (`/Game/Blueprints/bp_WarningLight.SpotLight1` _asbp_warning_light_4) 100000.0)
            (`LightComponent.SetLightColor` _spotlight_2 (struct :`R` 1.0 :`G` 1.0 :`B` 1.0 :`A` 1.0) true)
            (`LightComponent.SetLightColor` (`/Game/Blueprints/bp_WarningLight.SpotLight1` _asbp_warning_light_4) (struct :`R` 1.0 :`G` 1.0 :`B` 1.0 :`A` 1.0) true)))))
    (:`then_4`
      (`KismetSystemLibrary.Delay` 4.0)
      (for _array_element_5 _outactors
        (`|ExecutionSequence`
          (:`then_0`
            (bind _asbp_light_5 (cast `/Game/Blueprints/bp_Light` _array_element_5))
            (`LightComponent.SetIntensity` (`/Game/Blueprints/bp_Light.PointLight2` _asbp_light_5) 0.0))
          (:`then_1`
            (bind _asbp_warning_light_5 (cast `/Game/Blueprints/bp_WarningLight` _array_element_5))
            (`LightComponent.SetIntensity` (`/Game/Blueprints/bp_WarningLight.SpotLight1` _asbp_warning_light_5) 0.0)
            (`LightComponent.SetIntensity` (`/Game/Blueprints/bp_WarningLight.SpotLight` _asbp_warning_light_5) 0.0)))))
    (:`then_5`
      (`KismetSystemLibrary.Delay` 5.0)
      (for _array_element_6 _outactors
        (`|ExecutionSequence`
          (:`then_0`
            (bind _asbp_light_6 (cast `/Game/Blueprints/bp_Light` _array_element_6))
            (bind _pointlight2_3 (`/Game/Blueprints/bp_Light.PointLight2` _asbp_light_6))
            (`LightComponent.SetIntensity` _pointlight2_3 100000.0)
            (`LightComponent.SetLightColor` _pointlight2_3 (struct :`R` 1.0 :`A` 1.0) true)
            (`LightComponentBase.SetCastShadows` _pointlight2_3 false))
          (:`then_1`
            (bind _asbp_warning_light_6 (cast `/Game/Blueprints/bp_WarningLight` _array_element_6))
            (bind _spotlight_3 (`/Game/Blueprints/bp_WarningLight.SpotLight` _asbp_warning_light_6))
            (`LightComponent.SetIntensity` _spotlight_3 100000.0)
            (`LightComponent.SetIntensity` (`/Game/Blueprints/bp_WarningLight.SpotLight1` _asbp_warning_light_6) 100000.0)
            (`LightComponent.SetLightColor` _spotlight_3 (struct :`R` 1.0 :`A` 1.0) true)
            (`LightComponent.SetLightColor` (`/Game/Blueprints/bp_WarningLight.SpotLight1` _asbp_warning_light_6) (struct :`R` 1.0 :`A` 1.0) true)
            (`LightComponentBase.SetCastShadows` _spotlight_3 true)
            (`LightComponentBase.SetCastShadows` (`/Game/Blueprints/bp_WarningLight.SpotLight1` _asbp_warning_light_6) true)))))))

(fn `UserConstructionScript`)