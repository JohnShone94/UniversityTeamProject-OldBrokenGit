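; Main player character Blueprint that handles interaction and spawn placement.
; Interact checks overlap states: one replaces all widgets with a WorldSelector menu and pauses the game in UI-only mouse mode, the other calls Collect on power capsules tagged PlayerArea.
; BeginPlay and the Z key share a path that restarts the player at the PlayerStart named by the spawn point value.
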(event `InputAction|Interact`
  (params (Key :type "Key Structure" :default "AnyKey"))
  (bind _returnvalue (`GameplayStatics.GetPlayerController` 0))
  (:`Pressed`
    (`|ExecutionSequence`
      (:`then_0`
        (if (`self.GetIsOverlappingComp`)
          (`WidgetLayoutLibrary.RemoveAllWidgets`)
          (bind _returnvalue_2 (`|CreateWidget` "/Game/Blueprints/WorldSelector.WorldSelector_C"))
          (`UserWidget.AddToViewport` _returnvalue_2 0)
          (set `PlayerController.bShowMouseCursor` true _returnvalue)
          (`WidgetBlueprintLibrary.SetInputMode_UIOnlyEx` _returnvalue)
          (`GameplayStatics.SetGamePaused` true)))
      (:`then_1`
        (if (`self.GetIsOverlappingPower`)
          (bind _outactors (`GameplayStatics.GetAllActorsWithTag` (`self.PlayerArea`)))
          (for _array_element _outactors
            (bind _asbp_power_capsule (cast `/Game/Blueprints/bp_PowerCapsule` _array_element))
            (`/Game/Blueprints/bp_PowerCapsule.Collect` _asbp_power_capsule)))))))

(event `Key|Z`
  (params (Key :type "Key Structure" :default "AnyKey"))
  (bind _returnvalue (`GameplayStatics.GetPlayerController` 0))
  (bind _returnvalue_2 (`GameplayStatics.GetGameMode`))
  (:`Pressed`
    (`GameModeBase.RestartPlayerAtPlayerStart` _returnvalue_2 _returnvalue (`GameModeBase.K2_FindPlayerStart` _returnvalue_2 _returnvalue (`KismetStringLibrary.Conv_NameToString` (`self.GetSpawnPoint`))) :!label _label)))

(event `self.ReceiveBeginPlay`
  (goto _label))

(fn `UserConstructionScript`)