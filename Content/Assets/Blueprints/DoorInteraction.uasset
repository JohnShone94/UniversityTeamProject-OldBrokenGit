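; Door interaction trigger Blueprint that reacts to actors entering and leaving its overlap area.
; Begin and end overlap set an InTrigger flag, then share one branch that calls CallButtonTrue on entry or CallButtonFalse on exit.
; Both paths toggle a text render's visibility, flipping it on every overlap event without filtering which actor overlaps.
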(event `self.ReceiveActorBeginOverlap`
  (params (OtherActor :type "Actor Object Reference"))
  (set `self.InTrigger` true)
  (if (`self.InTrigger`) :!label _label
    (`SceneComponent.ToggleVisibility` (`self.TextRender`) false)
    (`self.ButtonTrue`)
    (else
      (`SceneComponent.ToggleVisibility` (`self.TextRender`) false)
      (`self.ButtonFalse`))))

(event `self.ReceiveActorEndOverlap`
  (params (OtherActor :type "Actor Object Reference"))
  (set `self.InTrigger` false)
  (goto _label))

(fn `UserConstructionScript`)